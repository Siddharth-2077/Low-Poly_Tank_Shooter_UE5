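; Toon Tanks game mode Blueprint that drives the UI for match start, player health and game over.
; StartGame puts the start widget and a stored health widget on screen, and UpdatePlayerHealth rewrites that widget's health text.
; GameOver uses a DoOnce so the end screen appears a single time, with win or loss text chosen by PlayerWon.
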(event EventStartGame
  ;[0.045 0.1094 0.07323 1 30] Start Game - Event
  (Development|PrintString "Start Game Event Called")
  (bind _returnvalue (UserInterface|CreateWidget "/Game/Blueprints/UI_Widgets/BP_StartGameWidget.BP_StartGameWidget_C"))
  (UserInterface|Viewport|AddtoViewport _returnvalue 0)
  (bind _returnvalue_2 (UserInterface|CreateWidget "/Game/Blueprints/UI_Widgets/BP_HealthWidget.BP_HealthWidget_C"))
  (bind _output_get (Variables|Default|SetHealthWidget _returnvalue_2))
  (UserInterface|Viewport|AddtoViewport _output_get 0))

(event EventGameOver
  (params (PlayerWon :type Boolean))
  ;[0.08854 0.04124 0.04058 1 30] Game Over - Event
  (Utilities|FlowControl|DoOnce false
    (:Completed
      (Development|PrintString "Game Over!")
      (bind _returnvalue (UserInterface|CreateWidget "/Game/Blueprints/UI_Widgets/BP_GameOverWidget.BP_GameOverWidget_C"))
      (UserInterface|Viewport|AddtoViewport _returnvalue 0)
      (if PlayerWon
        (Variables|/Script/UMG.TextBlock|SetText (Variables|/Game/Blueprints/UI_Widgets/BP_GameOverWidget.BP_GameOverWidget_C|GetDisplayText _returnvalue) "You Won!")
        (else
          (Variables|/Script/UMG.TextBlock|SetText (Variables|/Game/Blueprints/UI_Widgets/BP_GameOverWidget.BP_GameOverWidget_C|GetDisplayText _returnvalue) "You Lost!"))))))

(event EventUpdatePlayerHealth
  (params (HealthAmount :type Float%20%28single-precision%29))
  (bind _output_get (Variables|Default|SetHealthText "Health = "))
  (Rendering|Components|TextRender|SetText (Variables|/Game/Blueprints/UI_Widgets/BP_HealthWidget.BP_HealthWidget_C|GetPlayerHealthText (Variables|Default|GetHealthWidget)) (Utilities|Text|ToText(String) (Utilities|String|Append _output_get (Utilities|String|ToString(Float) HealthAmount)))))

(fn ConstructionScript)